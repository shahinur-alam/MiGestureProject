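; Gesture combination trainer for VR hand poses or motions that records samples, trains on them and tests recognition with debug prints.
; Each bone of the Hand mesh is one combination part, with strokes started relative to the VR pawn's camera.
; Tick feeds world-space bone transforms into active strokes and runs continuous identification, comparing average part similarity to a threshold.
; StopTrain launches training, and its finish callback saves the gesture database to file.
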(event `self.ReceiveBeginPlay`
  (`self.EnableInput` (`GameplayStatics.GetPlayerController` 0))
  (bind _asbp_vrpawn (cast `/Game/BP_VRPawn` (`self.Instigator`)))
  (set `self.VRCamera` (`/Game/BP_VRPawn.Camera` _asbp_vrpawn)))

(event `InitialiseGesture`
  (params (name :type String))
  (if (not (`self.bInitialised`))
    ;[1 1 1] Initialise
    (set `self.bInitialised` true)
    (bind _output_get (set `self.GestureName` name))
    (bind _returnvalue (`self.createGestureCombination` _output_get))
    (set `self.GestureIndex` _returnvalue)
    (bind _boneindex (`self.ForEachBone`)
      (:`Out`
        (bind _returnvalue_2 (`self.createGesture` _boneindex (`self.GestureName`)))
        (`self.setCombinationPartGesture` (`self.GestureIndex`) _boneindex _returnvalue_2))
      (:`Completed`
        (`KismetSystemLibrary.PrintString` "GESTURE INITIALISED" true true (struct :`G` 0.66 :`B` 1.0 :`A` 1.0) 10.0)))))

(event `StartTrain`
  ;[1 1 1] Start and stop training
  (if (`self.bInitialised`)
    (set `self.bTraining` true)
    (`KismetSystemLibrary.PrintString` "STARTED TRAINING" true true (struct :`G` 0.66 :`B` 1.0 :`A` 1.0) 10.0)))

(event `StopTrain`
  ;[1 1 1] Start and stop training
  (if (`self.bInitialised`)
    (if (`self.bStrokeRunning`)
      (`self.StopStroke`))
    (`self.startTraining`)
    (add `self.OnTrainingFinishDelegate` (delegate `OnTrainingFinished`))))

(event `OnTrainingFinished` :!signature `self.OnTrainingFinishDelegate`
  (params (Source :type "GestureCombinationsActor Object Reference") (Performance :type "Float (double-precision)"))
  ;[1 1 1] Start and stop training
  (`KismetSystemLibrary.PrintString` (`KismetStringLibrary.Concat_StrStr` "TRANING FINISHED, PERFORMANCE: " (`KismetStringLibrary.Conv_DoubleToString` Performance)))
  (bind _returnvalue (`self.saveToFile` (make `FilePath` (`self.DatabaseFileName`))))
  (if (== _returnvalue 0)
    (`KismetSystemLibrary.PrintString` "GESTURE SAVED TO DATABASE" true true (struct :`G` 0.66 :`B` 1.0 :`A` 1.0) 10.0)
    (set `self.bInitialised` false)
    (set `self.bTraining` false)
    (set `self.bStrokeRunning` false)
    (else
      (`KismetSystemLibrary.PrintString` (`KismetStringLibrary.Concat_StrStr` "Error: " (`MiVRyUtil.errorCodeToString` _returnvalue)) true true (struct :`G` 0.66 :`B` 1.0 :`A` 1.0) 20.0))))

(event `BeginStroke`
  (bind (_location _rotation) (`self.GetVRCameraTransform`))
  ;[1 1 1] Begin and end stroke
  (if (`self.bInitialised`)
    (if (not (`self.bStrokeRunning`))
      (bind _boneindex (`self.ForEachBone`)
        (:`Out`
          (`self.startStroke` _boneindex _location _rotation (`self.GestureIndex`)))
        (:`Completed`
          (set `self.bStrokeRunning` true)
          (`KismetSystemLibrary.PrintString` "STROKE BEGAN" true true (struct :`G` 0.66 :`B` 1.0 :`A` 1.0) 10.0))))))

(event `StopStroke`
  ;[1 1 1] Begin and end stroke
  (if (`self.bInitialised`)
    (if (`self.bStrokeRunning`)
      (bind _boneindex (`self.ForEachBone`)
        (:`Out`
          (`self.endStroke` _boneindex))
        (:`Completed`
          (set `self.bStrokeRunning` false)
          (`KismetSystemLibrary.PrintString` "STROKE FINISHED" true true (struct :`G` 0.66 :`B` 1.0 :`A` 1.0) 10.0))))))

(event `self.ReceiveTick`
  (params (DeltaSeconds :type "Float (single-precision)"))
  (bind (_location _rotation) (`self.GetVRCameraTransform`))
  (bind (_transform_location _transform_rotation) (`KismetMathLibrary.BreakTransform` (`self.Transform`)))
  (`|ExecutionSequence`
    (:`then_0`
      (if (or (and (`self.bTraining`) (`self.bStrokeRunning`)) (`self.bIdentifying`))
        (`|ExecutionSequence`
          (:`then_0`
            ;[1 1 1] Continue stroke
            (bind (_boneindex _bonename) (`self.ForEachBone`)
              (:`Out`
                (bind _returnvalue (`PoseableMeshComponent.GetBoneTransformByName` (`self.Hand`) _bonename "WorldSpace"))
                (bind _output_get (set `self.Transform` _returnvalue))
                (`self.contdStroke` _boneindex _transform_location _transform_rotation)))))))
    (:`then_1`
      ;[1 1 1] Continuous identification
      (if (`self.bIdentifying`)
        (bind (_similarity _partsprobabilities _partssimilarities _returnvalue_2) (`self.contdIdentify` _location _rotation))
        (if (>= _returnvalue_2 0)
          (bind _returnvalue_3 (`self.GetAverage` _partssimilarities))
          (`KismetSystemLibrary.PrintString` (`KismetStringLibrary.Conv_DoubleToString` _returnvalue_3))
          (if (> _returnvalue_3 (/ (`self.IdentifySimilarity`) 100.0))
            (bind _returnvalue_4 (`self.getGestureName` 0 _returnvalue_2))
            (`KismetSystemLibrary.PrintString` _returnvalue_4))
          (else
            (`KismetSystemLibrary.PrintString` (`KismetStringLibrary.Concat_StrStr` "Identification Failure: " (`MiVRyUtil.errorCodeToString` _returnvalue_2)))))))))

(event `IdentifyStartStroke`
  (bind (_location _rotation) (`self.GetVRCameraTransform`))
  (bind (_location_2 _rotation_2) (`self.GetVRCameraTransform`))
  ;[1 1 1] Identify start and stop stroke
  (if (not (`self.bIdentifying`))
    (set `self.CameraLocationCached` _location)
    (set `self.CameraRotationCached` _rotation)
    (bind _boneindex (`self.ForEachBone`)
      (:`Out`
        (`self.startStroke` _boneindex _location_2 _rotation_2)
        (`self.setContdIdentificationPeriod` _boneindex 4000))
      (:`Completed`
        (set `self.bIdentifying` true)))))

(event `IndetifyStopStroke`
  ;[1 1 1] Identify start and stop stroke
  (if (`self.bIdentifying`)
    (bind _boneindex (`self.ForEachBone`)
      (:`Out`
        (`self.endStroke` _boneindex))
      (:`Completed`
        (`KismetSystemLibrary.PrintString` "STOP IDENTIFY STROKE" true true (struct :`G` 0.66 :`B` 1.0 :`A` 1.0) 10.0)
        (set `self.bIdentifying` false)))))

(fn `GetAverage`
  (params (Values :type "Array of Float (double-precision)"))
  (returns (ReturnValue :type "Float (double-precision)"))
  (locals (Total :type "Float (double-precision)"))
  (for _array_element Values
    (set `local.Total` (+ (`local.Total`) _array_element)))
  (return (/ (`local.Total`) (`KismetMathLibrary.Conv_IntToDouble` (`KismetArrayLibrary.Array_Length` Values)))))

(fn `GetVRCameraTransform`
  (returns (Location :type "Vector Structure") (Rotation :type "Rotator Structure"))
  (return (`SceneComponent.K2_GetComponentLocation` (`self.VRCamera`)) (`SceneComponent.K2_GetComponentRotation` (`self.VRCamera`))))

(fn `UserConstructionScript`)